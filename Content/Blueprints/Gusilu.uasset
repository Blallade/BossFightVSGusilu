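; Gusilu is a boss enemy that bobs on a sine wave while patrolling a rectangle, alternating timeline-driven X/Y moves and yaw turns in an endless delay loop.
; Projectile overlaps on legs, head and rear deal increasing damage with distinct sounds.
; Tick brightens the head's dynamic material as HP falls.
; At zero HP, explosions repeat while music lowers, then the player's target resets and the boss is destroyed.
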(event OnComponentBeginOverlap(LegsCollision)
  (params (OverlappedComponent :type Primitive%20Component%20Object%20Reference) (OtherActor :type Actor%20Object%20Reference) (OtherComp :type Primitive%20Component%20Object%20Reference) (OtherBodyIndex :type Integer) (bFromSweep :type Boolean) (SweepResult :type Hit%20Result%20Structure%20%28by%20ref%29))
  ;[1 0.5312 0.5312] Collision damages
  (Utilities|Casting|CastToFirstPersonProjectile OtherActor)
  (Variables|Default|SetcurrentHP (- (Variables|Default|GetcurrentHP) 1.0))
  (Audio|PlaySoundatLocation "/Game/Audio/Slime.Slime" (Transformation|GetActorLocation) "0, 0, 0" 0.5 1.0 0.1 0 0 0))

(event OnComponentBeginOverlap(HeadCollision)
  (params (OverlappedComponent :type Primitive%20Component%20Object%20Reference) (OtherActor :type Actor%20Object%20Reference) (OtherComp :type Primitive%20Component%20Object%20Reference) (OtherBodyIndex :type Integer) (bFromSweep :type Boolean) (SweepResult :type Hit%20Result%20Structure%20%28by%20ref%29))
  ;[1 0.5312 0.5312] Collision damages
  (Utilities|Casting|CastToFirstPersonProjectile OtherActor)
  (Variables|Default|SetcurrentHP (- (Variables|Default|GetcurrentHP) 5.0))
  (Audio|PlaySoundatLocation "/Game/Audio/FaceSlap.FaceSlap" (Transformation|GetActorLocation) "0, 0, 0" 0.2 0.3 0.0 0 0 0))

(event OnComponentBeginOverlap(AssCollision)
  (params (OverlappedComponent :type Primitive%20Component%20Object%20Reference) (OtherActor :type Actor%20Object%20Reference) (OtherComp :type Primitive%20Component%20Object%20Reference) (OtherBodyIndex :type Integer) (bFromSweep :type Boolean) (SweepResult :type Hit%20Result%20Structure%20%28by%20ref%29))
  ;[1 0.5312 0.5312] Collision damages
  (Utilities|Casting|CastToFirstPersonProjectile OtherActor)
  (Variables|Default|SetcurrentHP (- (Variables|Default|GetcurrentHP) 5e+01))
  (Audio|PlaySoundatLocation "/Game/Audio/AAAAAH.AAAAAH" (Transformation|GetActorLocation) "0, 0, 0" 0.2 0.4 0.0 0 0 0))

(event Custom|RotateBoss
  ;[0.04314 1 0.1059] Moves the boss in the Z rotation.
  (if (not (Math|Float|NearlyEqual(Float) (Variables|Default|GetZRotation) 1.8e+02 1.0))
    (bind _alpha (Timeline|Timeline_0 PlayFromStart)
      (:Update
        (Transformation|SetWorldRotation (Variables|Default|GetDefaultSceneRoot) (Math|Rotator|MakeRotator 0.0 0.0 (Math|Float|Lerp (Variables|Default|GetZRotation) (- (Variables|Default|GetZRotation) 9e+01) _alpha)) false false))
      (:Finished
        (Variables|Default|SetZRotation (- (Variables|Default|GetZRotation) 9e+01))))
    (else
      (Variables|Default|SetZRotation -1.8e+02)
      (Timeline|Timeline_0 PlayFromStart))))

(event Custom|MoveBossStraight
  ;[0.04314 1 0.1059] Moves the boss in the X location
  (bind _alpha (Timeline|Timeline_1 PlayFromStart)
    (:Update
      (Transformation|SetRelativeLocation (Variables|Default|GetDefaultSceneRoot) (Math|Vector|MakeVector (Math|Float|Lerp (Variables|Default|GetXValue) (* (Variables|Default|GetXValue) -1.0) _alpha) (Variables|Default|GetYValue) (.z (Transformation|GetWorldLocation (Variables|Default|GetDefaultSceneRoot)))) false false))
    (:Finished
      (Variables|Default|SetXValue (* (Variables|Default|GetXValue) -1.0)))))

(event Custom|MoveBossLeft
  ;[0.04314 1 0.1059] Moves the boss in the Y location
  (bind _alpha (Timeline|Timeline_2 PlayFromStart)
    (:Update
      (Transformation|SetRelativeLocation (Variables|Default|GetDefaultSceneRoot) (Math|Vector|MakeVector (Variables|Default|GetXValue) (Math|Float|Lerp (Variables|Default|GetYValue) (* (Variables|Default|GetYValue) -1.0) _alpha) (.z (Transformation|GetWorldLocation (Variables|Default|GetDefaultSceneRoot)))) false false))
    (:Finished
      (Variables|Default|SetYValue (* (Variables|Default|GetYValue) -1.0)))))

(event Custom|BounceBoss
  (bind _returnvalue (Utilities|Time|GetWorldDeltaSeconds))
  (bind _returnvalue_2 (Actor|GetGameTimeSinceCreation))
  (bind _legsfloatingrange (Variables|Default|GetlegsFloatingRange))
  (bind _returnvalue_3 (* _returnvalue_2 1.0))
  (bind _returnvalue_4 (Math|Trig|Sin(Radians) _returnvalue_3))
  (bind _returnvalue_5 (* _returnvalue_4 _legsfloatingrange))
  (bind _returnvalue_6 (* _returnvalue _returnvalue_5))
  ;[1 0.4027 0.05604] Boss bouncing mechanic
  (Transformation|AddRelativeLocation (Variables|Default|GetLegs) (Math|Vector|MakeVector 0.0 0.0 _returnvalue_6) false false)
  (Transformation|AddRelativeLocation (Variables|Default|GetDefaultSceneRoot) (Math|Vector|MakeVector 0.0 0.0 (* _returnvalue_6 (Variables|Default|GetheadFloatingRange))) false false))

(event EventTick
  (params (DeltaSeconds :type Float%20%28single-precision%29))
  (bind _returnvalue (Game|GetPlayerCharacter 0))
  (bind _asfirst_person_character (Utilities|Casting|CastToFirstPersonCharacter _returnvalue))
  ;[0.05295 0.05663 0.6354] Change values when hp goes down
  (if (<= (Variables|Default|GetcurrentHP) 0.0)
    ;[0.03125 0 0] Death event
    (Utilities|FlowControl|Gate false :!label _label
      (:Exit
        (Utilities|FlowControl|Sequence
          (:then_0
            (Effects|SpawnEmitteratLocation "/Game/ThridParty/StarterContent/Particles/P_Explosion.P_Explosion" (Transformation|GetActorLocation) "0, 0, 0" "5.000000,5.000000,5.000000"))
          (:then_1
            (Utilities|FlowControl|DoOnce false
              (:Completed
                (bind _returnvalue_2 (Actor|GetActorOfClass "/Game/Blueprints/MusicManager.MusicManager_C"))
                (Default|MusicDown _returnvalue_2)
                (Utilities|FlowControl|Delay 4.0)
                (Utilities|FlowControl|Sequence
                  (:then_0
                    (Variables|/Game/Blueprints/FirstPersonCharacter.FirstPersonCharacter_C|SetenemyIsAlive? _asfirst_person_character false)
                    (Default|ResetTarget _asfirst_person_character)
                    (goto _label Close))
                  (:then_1
                    (Utilities|FlowControl|Delay 0.0001)
                    (Actor|DestroyActor)))))))))
    (else
      (CallFunction|BounceBoss)
      (Rendering|Material|SetScalarParameterValue (Variables|Default|GetDynamicHeadMat) "Emissive" (Math|Float|Lerp 0.1 0.0 (* (/ 1.0 (Variables|Default|Gethp)) (Variables|Default|GetcurrentHP))) :!class /Script/Engine.MaterialInstanceDynamic))))

(event EventBeginPlay
  (bind _defaultsceneroot (Variables|Default|GetDefaultSceneRoot))
  (bind _returnvalue (Transformation|GetWorldLocation _defaultsceneroot))
  ;[1 0.925 0.04934] Boss movement
  (Utilities|FlowControl|Delay 0.5)
  (Variables|Default|SetXValue (.x _returnvalue))
  (Variables|Default|SetYValue (.y _returnvalue))
  (Variables|Default|SetZRotation (.yaw (Transformation|GetWorldRotation _defaultsceneroot)))
  (CallFunction|MoveBossStraight :!label _label)
  (Utilities|FlowControl|Delay 1e+01)
  (CallFunction|RotateBoss)
  (Utilities|FlowControl|Delay 1.0)
  (CallFunction|MoveBossLeft)
  (Utilities|FlowControl|Delay 1e+01)
  (CallFunction|RotateBoss)
  (Utilities|FlowControl|Delay 1.0)
  (goto _label))

(fn ConstructionScript
  (bind _returnvalue (Rendering|Material|CreateDynamicMaterialInstance (Rendering|Material|GetMaterial (Variables|Default|GetHead) 0) "" "None" :!class /Script/Engine.KismetMaterialLibrary))
  (Variables|Default|SetDynamicHeadMat _returnvalue)
  (Rendering|Material|SetMaterial (Variables|Default|GetHead) 0 _returnvalue))